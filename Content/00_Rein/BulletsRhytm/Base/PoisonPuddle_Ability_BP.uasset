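; Rhythm-driven poison puddle ability actor that damages its surroundings and grows until it expires.
; On BeginPlay it caches the HealthComponent of its owning PoisonBomb_Ability and binds to the GM_Game beat event.
; Each beat damages every sphere-overlapping actor with a HealthComponent, increments a counter and uses a timeline to lerp uniform scale up to match it.
; The puddle destroys itself when the counter reaches BeatAmount.
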(event `self.ReceiveBeginPlay`
  (`|ExecutionSequence`
    (:`then_0`
      (bind _aspoison_bomb_ability (cast `/Game/00_Rein/BulletsRhytm/Base/PoisonBomb_Ability` (`self.GetOwner`)))
      (set `self.HealthComponent` (`/Game/0000_BulletsRhythm/Base/ProjectileBase.HealthComponent` _aspoison_bomb_ability)))
    (:`then_1`
      (set `self.SpawnTime` (`KismetMathLibrary.Now`))
      (add `/Game/0000_BulletsRhythm/Base/GM_Game.On_Beat` (cast `/Game/0000_BulletsRhythm/Base/GM_Game` (`GameplayStatics.GetGameMode`) :!pure true) (delegate `OnBeat`)))))

(event `OnBeat`
  (`self.PoisonDamage` null)
  (bind _output_get (set `self.CurrentBeatAmount` (+ (`self.CurrentBeatAmount`) 1)))
  (`self.ChangeScale`)
  (if (== _output_get (`self.BeatAmount`))
    (`self.K2_DestroyActor`)))

(event `ChangeScale`
  (bind _returnvalue (+ (`KismetMathLibrary.Conv_IntToDouble` (`self.CurrentBeatAmount`)) 1.0))
  (set `self.Scale` (`self.GetActorScale3D`))
  (bind (_direction _alpha) (`Timeline|ChangeScaleTimeline` :!via `PlayFromStart`)
    (:`Update`
      (`self.SetActorScale3D` (`KismetMathLibrary.VLerp` (`self.Scale`) (`KismetMathLibrary.MakeVector` _returnvalue _returnvalue _returnvalue) _alpha)))))

(event `PoisonDamage`
  (params (NewParam :type "Actor Object Reference"))
  (for _array_element (`PrimitiveComponent.GetOverlappingActors` (`self.Sphere`) "/Script/Engine.Actor")
    (bind _returnvalue (`self.GetComponentByClass` _array_element "/Game/0000_BulletsRhythm/Base/Health/HealthComponent.HealthComponent_C"))
    (`/Engine/EditorBlueprintResources/StandardMacros.IsValid` _returnvalue
      (:`Is Valid`
        (`/Game/0000_BulletsRhythm/Base/Health/HealthComponent.Damage` :`self` _returnvalue :`Damage` (`self.PoisonDamageAmount`))))))

(fn `UserConstructionScript`)