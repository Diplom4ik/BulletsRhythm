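; BulletBlink_Ability_BP is a short-lived ability actor that blinks the player character to the position of their weapon's referenced projectile.
; On BeginPlay it snapshots the player's location and the projectile's location, so the destination does not track the moving bullet.
; A timeline lerps the character between the two points without sweep collision, then the actor destroys itself.
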(event `self.ReceiveBeginPlay`
  (bind _asplayer_character (cast `/Game/0000_BulletsRhythm/Base/PlayerCharacter` (`GameplayStatics.GetPlayerCharacter` 0)))
  (set `self.PlayerCharacter` _asplayer_character)
  (set `self.StartLocation` (`self.K2_GetActorLocation` (`self.PlayerCharacter`)))
  (set `self.ProjectileLocation` (`self.K2_GetActorLocation` (`/Game/0000_BulletsRhythm/Base/WeaponBase.ProjectileReference` (`/Game/0000_BulletsRhythm/Base/PlayerCharacter.AWeapon` (`self.PlayerCharacter`)))))
  (bind (_direction _alpha) (`Timeline|Timeline_0` :!via `PlayFromStart`)
    (:`Update`
      (`self.K2_SetActorLocation` (`self.PlayerCharacter`) (`KismetMathLibrary.VLerp` (`self.StartLocation`) (`self.ProjectileLocation`) _alpha) false false))
    (:`Finished`
      (`self.K2_DestroyActor`))))

(fn `UserConstructionScript`)