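; Blueprint that drives a beat-synced post-process effect, changing the screen color on every music beat.
; On BeginPlay it creates a dynamic instance of BeatPostProcess_MAT and installs it as a weighted blendable on the referenced post process's settings.
; ChangeColor, called once at start and bound to GM_Game's OnBeat event, sets the material's Color parameter to the next entry in ColorArray, wrapping around.
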(event `self.ReceiveBeginPlay`
  (bind _returnvalue (`KismetMaterialLibrary.CreateDynamicMaterialInstance` "/Game/00_Rein/Materials/BeatPostProcess_MAT.BeatPostProcess_MAT"))
  (set `self.PostProcessMaterial` _returnvalue)
  (`KismetArrayLibrary.Array_Add` (`self.PostProcessMaterialsArray`) (make `WeightedBlendable` 1.0 (`self.PostProcessMaterial`)))
  ;[1 0.7292 0.9424] Set Material to Post Process
  (set `PostProcessVolume.Settings` (make `PostProcessSettings` :`WeightedBlendables` (make `WeightedBlendables` (`self.PostProcessMaterialsArray`))) (`self.PostProcessReference`))
  (`self.ChangeColor`)
  (add `/Game/0000_BulletsRhythm/Base/GM_Game.On_Beat` (cast `/Game/0000_BulletsRhythm/Base/GM_Game` (`GameplayStatics.GetGameMode`) :!pure true) (delegate `ChangeColor`)))

(event `ChangeColor`
  ;[1 0.7292 0.9424] Make the screen change color on every beat
  (set `self.CurrentColor` (`|GetArrayItem` (`self.ColorArray`) (`self.CurrentColorIndex`)))
  (`MaterialInstanceDynamic.SetVectorParameterValue` (`self.PostProcessMaterial`) "Color" (`self.CurrentColor`))
  (set `self.CurrentColorIndex` (mod (+ (`self.CurrentColorIndex`) 1) (`KismetArrayLibrary.Array_Length` (`self.ColorArray`)))))

(fn `UserConstructionScript`)