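; Sky sphere actor that changes its color in time with the game's beat.
; On BeginPlay it creates a dynamic material instance on the Sphere, applies the first color and binds ChangeColor to the OnBeat event of GM_Game.
; Each ChangeColor call sets the material's Color parameter from ColorArray, then advances the index, wrapping around to loop through the palette.
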(event `self.ReceiveBeginPlay`
  (bind _returnvalue (`PrimitiveComponent.CreateDynamicMaterialInstance` (`self.Sphere`) 0 (`PrimitiveComponent.GetMaterial` (`self.Sphere`) 0) "None"))
  (bind _output_get (set `self.SkyMaterial` _returnvalue))
  (`PrimitiveComponent.SetMaterial` (`self.Sphere`) 0 _output_get)
  (`self.ChangeColor`)
  (add `/Game/0000_BulletsRhythm/Base/GM_Game.On_Beat` (cast `/Game/0000_BulletsRhythm/Base/GM_Game` (`GameplayStatics.GetGameMode`) :!pure true) (delegate `ChangeColor`)))

(event `ChangeColor`
  ;[1 0.7292 0.9424] Make the sky change color on every beat
  (set `self.CurrentColor` (`|GetArrayItem` (`self.ColorArray`) (`self.CurrentColorIndex`)))
  (`MaterialInstanceDynamic.SetVectorParameterValue` (`self.SkyMaterial`) "Color" (`self.CurrentColor`))
  (set `self.CurrentColorIndex` (mod (+ (`self.CurrentColorIndex`) 1) (`KismetArrayLibrary.Array_Length` (`self.ColorArray`)))))

(fn `UserConstructionScript`)